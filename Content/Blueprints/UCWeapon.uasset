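; UCWeapon is a weapon base with base and alt actions, each playing a montage and sound behind a cooldown flag.
; PrivateBaseAction and PrivateAltAction are empty hooks for weapon-specific behavior.
; Tick counts cooldowns down in undilated time and matches audio pitch to global time dilation.
; As wired, AltAction calls PrivateBaseAction and resets BaseActionTime, leaving PrivateAltAction uncalled and AltActionTime never reset.
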(event EventTick
  (params (DeltaSeconds :type Float%20%28single-precision%29))
  (bind _returnvalue (Class|GameplayStatics|GetGlobalTimeDilation))
  (bind _returnvalue_2 (/ DeltaSeconds _returnvalue))
  (Audio|Components|Audio|SetPitchMultiplier (Variables|Default|GetBaseActionAudioComp) _returnvalue)
  (Utilities|FlowControl|Sequence
    (:then_0
      (if (not (Variables|Default|GetbCanPerformBaseAction))
        (if (< (- (Variables|Default|GetBaseActionTime) _returnvalue_2) 0.0)
          (Variables|Default|SetbCanPerformBaseAction true)
          (else
            (Variables|Default|SetBaseActionTime (- (Variables|Default|GetBaseActionTime) _returnvalue_2))))))
    (:then_1
      (if (not (Variables|Default|GetbCanPerformAltAction))
        (if (< (- (Variables|Default|GetAltActionTime) _returnvalue_2) 0.0)
          (Variables|Default|SetbCanPerformAltAction true)
          (else
            (Variables|Default|SetAltActionTime (- (Variables|Default|GetAltActionTime) _returnvalue_2))))))))

(fn ConstructionScript
  (Audio|Components|Audio|SetSound (Variables|Default|GetBaseActionAudioComp) (Variables|Default|GetBaseActionAudio))
  (Audio|Components|Audio|SetSound (Variables|Default|GetAltActionAudioComp) (Variables|Default|GetAltActionAudio)))

(fn BaseAction
  (params (inPawn :type Pawn%20Object%20Reference) (inSkelMeshComp :type Skeletal%20Mesh%20Component%20Object%20Reference))
  (if (Variables|Default|GetbCanPerformBaseAction)
    (bind _returnvalue (Animation|Montage|MontagePlay (Components|SkeletalMesh|GetAnimInstance inSkelMeshComp) (Variables|Default|GetBaseActionMontage) 1.0))
    (CallFunction|PrivateBaseAction inPawn)
    (Variables|Default|SetBaseActionTime (Variables|Default|GetBaseActionInterval))
    (Variables|Default|SetbCanPerformBaseAction false)
    (Audio|Components|Audio|Play (Variables|Default|GetBaseActionAudioComp) 0.0)
    (return _returnvalue)))

(fn PrivateBaseAction
  (params (inPawn :type Pawn%20Object%20Reference)))

(fn AltAction
  (params (inPawn :type Pawn%20Object%20Reference) (inSkelMeshComp :type Skeletal%20Mesh%20Component%20Object%20Reference))
  (if (Variables|Default|GetbCanPerformAltAction)
    (bind _returnvalue (Animation|Montage|MontagePlay (Components|SkeletalMesh|GetAnimInstance inSkelMeshComp) (Variables|Default|GetAltActionMontage) 1.0))
    (CallFunction|PrivateBaseAction inPawn)
    (Variables|Default|SetBaseActionTime (Variables|Default|GetAltActionInterval))
    (Variables|Default|SetbCanPerformAltAction false)
    (Audio|Components|Audio|Play (Variables|Default|GetAltActionAudioComp) 0.0)
    (return _returnvalue)))

(fn PrivateAltAction
  (params (inPawn :type Pawn%20Object%20Reference) (inSkelMeshComp :type Skeletal%20Mesh%20Component%20Object%20Reference)))