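; Shotgun pickup actor that grants the player a shotgun when walked over.
; When MyCharacter overlaps its Box1 trigger, it turns off its particle effect and destroys the trigger so it fires only once.
; It then switches the character's gun, sets its ammo from the Ammo variable, shows a "+ Shotgun" instruction and plays a loading sound at the pickup.
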(event OnComponentBeginOverlap(Box1)
  (params (OtherActor :type Actor%20Object%20Reference) (OtherComp :type Primitive%20Component%20Object%20Reference) (OtherBodyIndex :type Integer) (bFromSweep :type Boolean) (SweepResult :type Hit%20Result%20Structure%20%28by%20ref%29))
  ;[1 1 1] Pick up shotgun
  (bind _asmycharacter_c (Utilities|Casting|CastToMyCharacter OtherActor))
  (Components|Activation|Deactivate (Variables|Default|GetParticleSystem1))
  (Components|DestroyComponent (Variables|Default|GetBox1))
  (Default|SwitchGuns _asmycharacter_c)
  (Default|SetAmmo _asmycharacter_c (Variables|Default|GetAmmo))
  (Default|DisplayInstruction _asmycharacter_c "+ Shotgun")
  (Audio|PlaySoundatLocation "/Game/Audio/Weapon/loadingWeapon.loadingWeapon" (Transformation|GetActorLocation)))

(fn ConstructionScript)