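; UCWeaponRanged is a ranged weapon Blueprint that adds ammo handling to a weapon action.
; BaseAction, gated by an interval, plays a montage, then either spends a round and calls the empty PrivateBaseAction hook or plays a no-ammo sound.
; AddAmmo always plays its sound but only adds a round up to MaxAmmo.
; Tick matches both ammo sounds' pitch to global time dilation.
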(event EventTick
  (params (DeltaSeconds :type Float%20%28single-precision%29))
  (|CallParentFunction DeltaSeconds)
  (Audio|Components|Audio|SetPitchMultiplier (Variables|Default|GetNoAmmoAudioComp) (Class|GameplayStatics|GetGlobalTimeDilation)))

(event EventPrivateBaseAction
  (params (inPawn :type Pawn%20Object%20Reference))
  ;[1 1 1] Check ammo
)

(fn ConstructionScript
  (|CallParentFunction))

(fn AddAmmo
  (Audio|Components|Audio|Play (Variables|Default|GetAddAmmoAudioComp) 0.0)
  (if (<= (+ (Variables|Default|GetAmmo) 1) (Variables|Default|GetMaxAmmo))
    (Variables|Default|SetAmmo (+ (Variables|Default|GetAmmo) 1))
    (LocalVariables|SetbAdded true)
    (return (LocalVariables|GetbAdded))
    (else
      (LocalVariables|SetbAdded false))))

(fn BaseAction
  (params (inPawn :type Pawn%20Object%20Reference) (inSkelMeshComp :type Skeletal%20Mesh%20Component%20Object%20Reference))
  (if (Variables|Default|GetbCanPerformBaseAction)
    (bind _returnvalue (Animation|Montage|MontagePlay (Components|SkeletalMesh|GetAnimInstance inSkelMeshComp) (Variables|Default|GetBaseActionMontage) 1.0))
    (Variables|Default|SetBaseActionTime (Variables|Default|GetBaseActionInterval))
    (Variables|Default|SetbCanPerformBaseAction false)
    ;[1 1 1] Check ammo
    (if (> (Variables|Default|GetAmmo) 0)
      (Variables|Default|SetAmmo (- (Variables|Default|GetAmmo) 1))
      (Audio|Components|Audio|Play (Variables|Default|GetBaseActionAudioComp) 0.0)
      (CallFunction|PrivateBaseAction inPawn)
      (return _returnvalue)
      (else
        (Audio|Components|Audio|Play (Variables|Default|GetNoAmmoAudioComp) 0.0)))))