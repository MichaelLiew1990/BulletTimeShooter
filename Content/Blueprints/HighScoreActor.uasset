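; Level actor that tracks the best completion time for a level and shows it on the HUD.
; On BeginPlay it enables the HUD high score display and loads a HighScoreSave from its slot, or creates one with a default score.
; CheckForLevelRecord stops the character's timer, stores the elapsed time in the game instance's LevelTimes, and saves and displays it if it beats the record.
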(event Custom|CheckForLevelRecord
  (bind _highscoreobject (Variables|Default|GetHighScoreObject))
  ;[1 1 1] Should be called when player has completed the level and you want to stop timer and check if the record was beaten.
  (bind _asmycharacter_c (Utilities|Casting|CastToMyCharacter (Game|GetPlayerCharacter 0)))
  (Variables|/Game/Blueprints/MyCharacter.MyCharacter_C|SetbUseTimer _asmycharacter_c false)
  (bind _asucgameinstance_c (Utilities|Casting|CastToUCGameInstance (Game|GetGameInstance)))
  (Utilities|Array|SetArrayElem (Variables|/Game/Blueprints/UCGameInstance.UCGameInstance_C|GetLevelTimes _asucgameinstance_c) (Variables|Default|GetLevelIndex) (Variables|/Game/Blueprints/MyCharacter.MyCharacter_C|GetElapsedLevelTime _asmycharacter_c))
  (if (< (Variables|/Game/Blueprints/MyCharacter.MyCharacter_C|GetElapsedLevelTime _asmycharacter_c) (Variables|/Game/Blueprints/HighScoreSave.HighScoreSave_C|GetHighScore _highscoreobject))
    (Variables|/Game/Blueprints/HighScoreSave.HighScoreSave_C|SetHighScore _highscoreobject (Variables|/Game/Blueprints/MyCharacter.MyCharacter_C|GetElapsedLevelTime _asmycharacter_c))
    (SaveGame|SaveGametoSlot (Variables|Default|GetHighScoreObject) (Utilities|String|ToString(Name) (Variables|Default|GetSaveSlotName)))
    (bind _asmyhud_c (Utilities|Casting|CastToMyHUD (HUD|GetHUD (Game|GetPlayerController 0))))
    (Variables|/Game/Blueprints/MyHUD.MyHUD_C|SetCurrentHighScore _asmyhud_c (Variables|/Game/Blueprints/HighScoreSave.HighScoreSave_C|GetHighScore (Variables|Default|GetHighScoreObject)))))

(event EventBeginPlay
  ;[1 1 1] BeginPlay and Initialize variables. Tell HUD to actually draw timer and load best score for this level
  (bind _asmyhud_c (Utilities|Casting|CastToMyHUD (HUD|GetHUD (Game|GetPlayerController 0))))
  (Variables|/Game/Blueprints/MyHUD.MyHUD_C|SetbDrawHighScore _asmyhud_c true)
  (bind _returnvalue (SaveGame|DoesSaveGameExist (Utilities|String|ToString(Name) (Variables|Default|GetSaveSlotName))))
  (if _returnvalue
    (bind _returnvalue_2 (SaveGame|LoadGamefromSlot (Utilities|String|ToString(Name) (Variables|Default|GetSaveSlotName))))
    (bind _ashighscoresave_c (Utilities|Casting|CastToHighScoreSave _returnvalue_2))
    (Variables|Default|SetHighScoreObject _ashighscoresave_c)
    (else
      (bind _returnvalue_3 (SaveGame|CreateSaveGameObject "/Game/Blueprints/HighScoreSave.HighScoreSave_C"))
      (bind _ashighscoresave_c_2 (Utilities|Casting|CastToHighScoreSave _returnvalue_3))
      (Variables|Default|SetHighScoreObject _ashighscoresave_c_2)
      (Variables|/Game/Blueprints/HighScoreSave.HighScoreSave_C|SetHighScore (Variables|Default|GetHighScoreObject) (Variables|Default|GetDefaultHighScore))))
  (bind _asmyhud_c_2 (Utilities|Casting|CastToMyHUD (HUD|GetHUD (Game|GetPlayerController 0))))
  (Variables|/Game/Blueprints/MyHUD.MyHUD_C|SetCurrentHighScore _asmyhud_c_2 (Variables|/Game/Blueprints/HighScoreSave.HighScoreSave_C|GetHighScore (Variables|Default|GetHighScoreObject))))

(fn ConstructionScript)