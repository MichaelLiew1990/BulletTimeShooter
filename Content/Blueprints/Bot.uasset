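; Enemy bot that spawns a gun at its hand socket, targets the player, and can be killed by bullets or knife stabs.
; A looping timer line-traces from the head to find players in range, while Tick turns toward the target and sets line-of-sight by dot product.
; An AnimNotify triggers shooting.
; Hits spawn blood, and lethal ones trigger ragdoll with impulse, then a timeline material dissolve before the actor is destroyed.
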(event Custom|Shoot
  (bind _targetactor (Variables|Default|GetTargetActor))
  ;[1 1 1] Shoot (this is called from AnimBlueprint only using AnimNotify!)
  ;;[1 1 1] Shoot only if my target is still valid and if I'm alive
  (if (!= _targetactor 0)
    (if (> (Variables|Default|GetHitPoints) 0)
      (Default|BotShot (Variables|Default|GetWeapon) _targetactor self))))

(event Custom|Closegate
  (bind _skeletalmesh1 (Variables|Default|GetSkeletalMesh1))
  (bind _skeletalmesh1_2 (Variables|Default|GetSkeletalMesh1))
  ;[1 1 1] OnHit (by bullet). Always reduce health and spawn blood particle, if the shot was lethal, enable ragdoll, add impulse and start dissolve material sequence. When Material is invisible disable collision and destroy actor
  (Utilities|FlowControl|Gate false) ; enters at Close
)

(event Custom|OnStabbed
  (params (ImpactLocation :type Vector) (ImpactNormal :type Vector) (BoneName :type Name))
  (bind _skeletalmesh1 (Variables|Default|GetSkeletalMesh1))
  (bind _skeletalmesh1_2 (Variables|Default|GetSkeletalMesh1))
  ;[1 1 1] Called when player stabs me. Knife deals 2 damage! Always spawn particle blood effect and If it kills me, enable ragdoll and add impulse
  (Variables|Default|SetHitPoints (- (Variables|Default|GetHitPoints) 2))
  (Effects|SpawnEmitteratLocation "/Game/Particles/P_body_bullet_impact.P_body_bullet_impact" ImpactLocation (Math|Conversions|RotationFromXVector ImpactNormal))
  (if (not (> (Variables|Default|GetHitPoints) 0))
    (Class|SkeletalMeshComponent|SetAllBodiesBelowSimulatePhysics _skeletalmesh1_2 (Class|SkinnedMeshComponent|GetBoneName _skeletalmesh1_2 1) true true)
    (Physics|AddImpulseatLocation _skeletalmesh1_2 (* ImpactNormal -7.5e+03) ImpactLocation BoneName)
    ;[1 1 1] OnHit (by bullet). Always reduce health and spawn blood particle, if the shot was lethal, enable ragdoll, add impulse and start dissolve material sequence. When Material is invisible disable collision and destroy actor
    (Utilities|FlowControl|Sequence
      (:then_0
        ;;[1 1 1] Dissolve material effect when I'm dead
        (bind _opacity (Timeline|DissolveTimeline PlayFromStart)
          (:Update
            (Rendering|Material|SetScalarParameterValue (Variables|Default|GetMatInst) "Opacity" _opacity :!class /Script/Engine.MaterialInstanceDynamic))
          (:Finished
            (Rendering|SetActorHiddenInGame true)
            (Collision|SetActorEnableCollision false)
            (Class|SkeletalMeshComponent|SetAllBodiesBelowSimulatePhysics _skeletalmesh1 (Class|SkinnedMeshComponent|GetBoneName _skeletalmesh1 1) false true)
            (Utilities|Time|ClearTimerbyFunctionName self "CheckForPlayer")
            (Actor|DestroyActor))))
      (:then_1
        (CallFunction|Closegate)))))

(event EventTick
  (params (DeltaSeconds :type Float%20%28single-precision%29))
  (bind _returnvalue (Transformation|GetActorRotation))
  (bind _desiredrotation (Variables|Default|GetDesiredRotation))
  (bind _yaw (Math|Rotator|BreakRotator _returnvalue))
  (bind _yaw_2 (Math|Rotator|BreakRotator _desiredrotation))
  ;[1 1 1] Tick
  ;;[1 1 1] Only check further if I'm alive
  (if (> (Variables|Default|GetHitPoints) 0)
    (if (or (!= _yaw _yaw_2) (== _yaw_2 _yaw))
      (if (!= (Variables|Default|GetTargetActor) 0)
        (Variables|Default|SetbLockTimer true)
        (Transformation|SetActorRotation (Math|Rotator|Lerp(Rotator) (Transformation|GetActorRotation) (Math|Rotator|MakeRotator 0.0 0.0 _yaw_2) (* DeltaSeconds (Variables|Default|GetRotationRate)) true))
        (Variables|Default|SetbHasLOS (> (Math|Vector|DotProduct (Math|Vector|Normalize (Math|Rotator|GetRotationXVector (Transformation|GetActorRotation))) (Math|Vector|Normalize (Class|KismetMathLibrary|GetDirectionVector (Transformation|GetActorLocation) (Transformation|GetActorLocation (Variables|Default|GetTargetActor))))) 0.85))
        (Variables|Default|SetbLockTimer false)
        (else
          (Variables|Default|SetbHasLOS false :!label _label)
          (Variables|Default|SetbLockTimer false)))
      (else
        (goto _label)))
    (else
      (goto _label))))

(event EventBeginPlay
  (bind _skeletalmesh1 (Variables|Default|GetSkeletalMesh1))
  ;[1 1 1] BeginPlay
  (Utilities|FlowControl|Delay 0.5)
  (Utilities|Time|SetTimerbyFunctionName self "CheckForPlayer" 0.1 true)
  ;[1 1 1] Spawn weapon
  (bind _returnvalue (Game|SpawnActorfromClass "/Game/Blueprints/UCWeapon_BotGun.UCWeapon_BotGun_C" (Transformation|GetSocketTransform _skeletalmesh1 "b_Gun" "RTS_World") "AdjustIfPossibleButDontSpawnIfColliding" 0 0))
  (Variables|Default|SetWeapon _returnvalue)
  (Class|Actor|AttachRootComponentto _returnvalue _skeletalmesh1 "b_Gun" "KeepWorldPosition" true))

(event Collision|EventHit
  (params (MyComp :type Primitive%20Component%20Object%20Reference) (Other :type Actor%20Object%20Reference) (OtherComp :type Primitive%20Component%20Object%20Reference) (bSelfMoved :type Boolean) (HitLocation :type Vector :default "0, 0, 0") (HitNormal :type Vector :default "0, 0, 0") (NormalImpulse :type Vector :default "0, 0, 0") (Hit :type Hit%20Result%20Structure%20%28by%20ref%29))
  (bind (_bblockinghit _binitialoverlap _time _location _impactpoint _normal _impactnormal _physmat _hitactor _hitcomponent _hitbonename) (Collision|BreakHitResult Hit))
  (bind _skeletalmesh1 (Variables|Default|GetSkeletalMesh1))
  (bind _skeletalmesh1_2 (Variables|Default|GetSkeletalMesh1))
  ;[1 1 1] OnHit (by bullet). Always reduce health and spawn blood particle, if the shot was lethal, enable ragdoll, add impulse and start dissolve material sequence. When Material is invisible disable collision and destroy actor
  (Utilities|FlowControl|Gate false
    (:Exit
      (Utilities|Casting|CastToUCProjectile Other)
      (Utilities|FlowControl|Sequence
        (:then_0
          (Variables|Default|SetHitPoints (- (Variables|Default|GetHitPoints) 1))
          (if (not (> (Variables|Default|GetHitPoints) 0))
            (Utilities|Time|ClearTimerbyFunctionName self "CheckForPlayer")
            (Class|SkeletalMeshComponent|SetAllBodiesBelowSimulatePhysics _skeletalmesh1_2 (Class|SkinnedMeshComponent|GetBoneName _skeletalmesh1_2 1) true true)
            (Physics|AddImpulseatLocation _skeletalmesh1_2 (* _impactnormal -7.5e+03) _impactpoint _hitbonename)
            (Utilities|FlowControl|Sequence
              (:then_0
                ;;[1 1 1] Dissolve material effect when I'm dead
                (bind _opacity (Timeline|DissolveTimeline PlayFromStart)
                  (:Update
                    (Rendering|Material|SetScalarParameterValue (Variables|Default|GetMatInst) "Opacity" _opacity :!class /Script/Engine.MaterialInstanceDynamic))
                  (:Finished
                    (Rendering|SetActorHiddenInGame true)
                    (Collision|SetActorEnableCollision false)
                    (Class|SkeletalMeshComponent|SetAllBodiesBelowSimulatePhysics _skeletalmesh1 (Class|SkinnedMeshComponent|GetBoneName _skeletalmesh1 1) false true)
                    (Utilities|Time|ClearTimerbyFunctionName self "CheckForPlayer")
                    (Actor|DestroyActor))))
              (:then_1
                (CallFunction|Closegate)))))
        (:then_1
          (Effects|SpawnEmitteratLocation "/Game/Particles/P_body_bullet_impact.P_body_bullet_impact" HitLocation (Math|Conversions|RotationFromXVector HitNormal)))))))

(fn ConstructionScript
  (bind _skeletalmesh1 (Variables|Default|GetSkeletalMesh1))
  (bind _returnvalue (Rendering|Material|CreateDynamicMaterialInstance _skeletalmesh1 0 "/Game/Materials/M_TestMat.M_TestMat" :!class /Script/Engine.PrimitiveComponent))
  (Variables|Default|SetMatInst _returnvalue)
  (Rendering|Material|SetMaterial _skeletalmesh1 0 (Variables|Default|GetMatInst)))

(fn CheckforPlayer
  (bind _returnvalue (Game|GetPlayerCharacter 0))
  (bind _asmy_character (Utilities|Casting|CastToMyCharacter _returnvalue))
  (bind _outhit (Collision|LineTraceByChannel (.Location (Math|Transform|BreakTransform (Transformation|GetSocketTransform (Variables|Default|GetSkeletalMesh1) "headSocket" "RTS_World"))) (+ (Transformation|GetActorLocation _returnvalue) (Variables|/Script/Engine.SceneComponent|GetRelativeLocation (Variables|/Game/Blueprints/MyCharacter.MyCharacter_C|GetFirstPersonCamera _asmy_character))) "TraceTypeQuery2" false 0 "None"))
  (if (!= (.HitActor (Collision|BreakHitResult _outhit)) 0)
    (if (== (.HitActor (Collision|BreakHitResult _outhit)) _returnvalue)
      (if (< (Transformation|GetDistanceTo (.HitActor (Collision|BreakHitResult _outhit))) (Variables|Default|GetRange))
        (Variables|Default|SetDesiredRotation (Math|Rotator|FindLookatRotation (Transformation|GetActorLocation) (Transformation|GetActorLocation (.HitActor (Collision|BreakHitResult _outhit)))))
        (Variables|Default|SetTargetActor (.HitActor (Collision|BreakHitResult _outhit)))
        (else
          (if (not (Variables|Default|GetbLockTimer)) :!label _label
            (Variables|Default|SetTargetActor 0))))
      (else
        (goto _label)))))