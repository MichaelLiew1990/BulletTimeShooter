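; Game instance that manages the game's screen states: playing, pause, main menu, credits, death and level end.
; Each event sets ScreenState and toggles game pause, input mode and cursor, with StartPlay reloading the current level and ToggleMainMenu opening the menu level.
; The level-end event waits briefly, then writes the character's elapsed time to the HUD's end-level widget.
; SetLevelTime stores that time per level index.
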(event Custom|EnableCredits
  ;[1 1 1] Enable credits menu. Disable player input and pause the game. Proper widget will be added via HUD
  (Variables|Default|SetScreenState "NewEnumerator4")
  (Game|SetGamePaused true)
  (Input|SetInputModeUIOnly 0 0 false)
  (Variables|/Script/Engine.PlayerController|SetbShowMouseCursor (Game|GetPlayerController 0) true))

(event Custom|EnableEndLevelMenu
  (bind _returnvalue (Game|GetPlayerController 0))
  ;[1 1 1] Enable End Level screen. Set a small delay and pause the game, switch input to UI only mode and update high score UI
  (Utilities|FlowControl|Delay 2.0)
  (Variables|Default|SetScreenState "NewEnumerator5")
  (Game|SetGamePaused true)
  (Input|SetInputModeUIOnly _returnvalue 0 false)
  (bind _asmyhud_c (Utilities|Casting|CastToMyHUD (HUD|GetHUD _returnvalue)))
  (bind _asmycharacter_c (Utilities|Casting|CastToMyCharacter (Game|GetPlayerCharacter 0)))
  (Rendering|Components|TextRender|SetText (Variables|/Game/UI/EndLevelWidget.EndLevelWidget_C|GetLevelTimetext (Variables|/Game/Blueprints/MyHUD.MyHUD_C|GetEndLevelWidget _asmyhud_c)) (Utilities|Text|ToText(Float) (Variables|/Game/Blueprints/MyCharacter.MyCharacter_C|GetElapsedLevelTime _asmycharacter_c) "HalfToEven" true 1 324 2 2))
  (Variables|/Script/Engine.PlayerController|SetbShowMouseCursor _returnvalue true))

(event Custom|ToggleMainMenu
  (bind _returnvalue (Game|GetPlayerController 0))
  ;[1 1 1] Toggle Main Menu mode. Disable player input, remove widgets from the HUD and switch to MainMenuLevel
  (Variables|Default|SetScreenState "NewEnumerator2")
  (Game|SetGamePaused true)
  (Input|SetInputModeUIOnly _returnvalue 0 false)
  (bind _asmyhud_c (Utilities|Casting|CastToMyHUD (HUD|GetHUD _returnvalue)))
  (Default|RemoveGameHUDWidget _asmyhud_c)
  (Variables|/Script/Engine.PlayerController|SetbShowMouseCursor _returnvalue true)
  (Game|OpenLevel(byName) "TestMainMenu"))

(event Custom|EnableDieMenu
  (bind _returnvalue (Game|GetPlayerController 0))
  ;[1 1 1] Switch game mode to 'PlayerDied'. Pause the game and show mouse cursor so player can navigate through DieMenu
  (Variables|Default|SetScreenState "NewEnumerator3")
  (Game|SetGamePaused true)
  (Input|SetInputModeUIOnly _returnvalue 0 false)
  (Variables|/Script/Engine.PlayerController|SetbShowMouseCursor _returnvalue true))

(event Custom|TogglePauseMenu
  (bind _returnvalue (Game|GetPlayerController 0))
  (bind _returnvalue_2 (Game|GetPlayerController 0))
  ;[1 1 1] Toggle Pause menu.
  (switch Utilities|FlowControl|Switch|SwitchonUCGameState (Variables|Default|GetScreenState)
    (:NewEnumerator0
      (Variables|Default|SetScreenState "NewEnumerator1")
      (Game|SetGamePaused false)
      (Input|SetInputModeGameOnly _returnvalue)
      (Variables|/Script/Engine.PlayerController|SetbShowMouseCursor _returnvalue false))
    (:NewEnumerator1
      (Variables|Default|SetScreenState "NewEnumerator0" :!label _label)
      (Game|SetGamePaused true)
      (Input|SetInputModeUIOnly _returnvalue_2 0 false)
      (Variables|/Script/Engine.PlayerController|SetbShowMouseCursor _returnvalue_2 true))
    (:NewEnumerator2
      (goto _label))
    (:NewEnumerator3
      (goto _label))))

(event Custom|StartPlay
  (bind _returnvalue (Game|GetPlayerController 0))
  ;[1 1 1] Call it if you want to restart the level. Enable player input and unpouse the game.
  (Class|WidgetBlueprintLibrary|SetFocustoGameViewport)
  (Variables|Default|SetScreenState "NewEnumerator1")
  (Game|SetGamePaused false)
  (Input|SetInputModeGameOnly _returnvalue)
  (Variables|/Script/Engine.PlayerController|SetbShowMouseCursor _returnvalue false)
  (Game|OpenLevel(byName) (Variables|Default|GetCurrentLevelName)))

(fn SetUCScreenState
  (params (NewState :type UCGameState%20Enum)))

(fn SetLevelTime
  (params (inLevelIndex :type Integer))
  (if (< inLevelIndex (Utilities|Array|Length (Variables|Default|GetLevelTimes)))
    (bind _asmycharacter_c (Utilities|Casting|CastToMyCharacter (Game|GetPlayerCharacter 0)))
    (Utilities|Array|SetArrayElem (Variables|Default|GetLevelTimes) inLevelIndex (Variables|/Game/Blueprints/MyCharacter.MyCharacter_C|GetElapsedLevelTime _asmycharacter_c))))